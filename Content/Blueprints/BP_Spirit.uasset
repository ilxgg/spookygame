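; BP_Spirit is a spirit actor with a Paper2D sprite that blinks in and out of view.
; A looping one-second timer started on BeginPlay drives a FlipFlop that alternately hides and shows the sprite.
; Every tick, the Arrow component turns in yaw only to face the first player's camera, a billboard-style rotation.
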(event Custom|Phase
  (bind _papersprite (Variables|Default|GetPaperSprite))
  (Utilities|FlowControl|FlipFlop
    (:A
      (Rendering|SetVisibility _papersprite false false))
    (:B
      (Rendering|SetVisibility _papersprite true false))))

(event EventBeginPlay
  (Utilities|Time|SetTimerbyEvent (delegate Custom|Phase) 1.0 true))

(event Collision|EventActorBeginOverlap
  (params (OtherActor :type Actor%20Object%20Reference)))

(event EventTick
  (params (DeltaSeconds :type Float%20%28single-precision%29))
  (bind _arrow (Variables|Default|GetArrow))
  (Transformation|SetWorldRotation _arrow (Math|Rotator|MakeRotator 0.0 0.0 (.yaw (Math|Rotator|FindLookatRotation (Transformation|GetWorldLocation _arrow) (Camera|GetCameraLocation (Variables|/Script/Engine.PlayerController|GetPlayerCameraManager (Game|GetPlayerController 0)))))) false false))

(fn ConstructionScript)