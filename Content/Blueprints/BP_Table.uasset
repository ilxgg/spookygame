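; BP_Table is an interactable table that shows paged dialogue through a WBP_InteractionDialogue widget.
; The first OnInteract creates the widget, shows the first Text entry and blocks player move and look input.
; Later interactions advance the page until a hard-coded limit, then remove the widget, restore input and reset the state.
; BeginPlay enables input, but the Continue action only checks the dialogue flag without acting.
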(event Collision|EventActorBeginOverlap
  (params (OtherActor :type Actor%20Object%20Reference)))

(event EventTick
  (params (DeltaSeconds :type Float%20%28single-precision%29)))

(event EventOnInteract
  (if (Variables|Default|GetDialogueTable)
    (CallFunction|NextDialogue)
    (else
      (CallFunction|TableDialogue))))

(event EventBeginPlay
  (Input|EnableInput (Game|GetPlayerController 0)))

(event Input|ActionEvents|InputActionContinue
  (params (Key :type Key%20Structure :default "None"))
  (:Pressed
    (if (Variables|Default|GetDialogueTable)
      _)))

(fn ConstructionScript)

(fn TableDialogue
  (bind _returnvalue (Game|GetPlayerController 0))
  (Variables|Default|SetDialogueTable true)
  (Variables|Default|SetDialoguePage 0)
  (bind _returnvalue_2 (UserInterface|CreateWidget "/Game/UI/Widgets/WBP_InteractionDialogue.WBP_InteractionDialogue_C"))
  (bind _output_get (Variables|Default|SetDialogueUI _returnvalue_2))
  (UserInterface|Viewport|AddtoViewport _output_get 0)
  (Variables|/Game/UI/Widgets/WBP_InteractionDialogue.WBP_InteractionDialogue_C|SetDialogueText _output_get (Utilities|Array|Get(acopy) (Variables|Default|GetText) (Variables|Default|GetDialoguePage)))
  (Input|SetIgnoreMoveInput _returnvalue true)
  (Input|SetIgnoreLookInput _returnvalue true))

(fn NextDialogue
  (bind _returnvalue (Game|GetPlayerController 0))
  (bind _dialogueui (Variables|Default|GetDialogueUI))
  (Variables|Default|SetDialoguePage (+ (Variables|Default|GetDialoguePage) 1))
  (Development|PrintString (Utilities|String|ToString(Integer) (Variables|Default|GetDialoguePage)))
  (Variables|/Game/UI/Widgets/WBP_InteractionDialogue.WBP_InteractionDialogue_C|SetDialogueText _dialogueui (Utilities|Array|Get(acopy) (Variables|Default|GetText) (Variables|Default|GetDialoguePage)))
  (if (>= (Variables|Default|GetDialoguePage) 2)
    (Widget|RemovefromParent _dialogueui)
    (Input|ResetIgnoreMoveInput _returnvalue)
    (Input|ResetIgnoreLookInput _returnvalue)
    (Variables|Default|SetDialoguePage 0)
    (Variables|Default|SetDialogueTable false)))