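; Ghost actor for a scripted haunting in which it walks a spline path, by its event name down stairs, then vanishes.
; Its skeletal mesh and terror radius stay hidden from BeginPlay until GhostWalkDownStairs reveals them.
; That event plays the MovePath timeline, scaled by Duration and started at MovementOffset, to set location and rotation along the referenced Spline's Pathway.
; The actor destroys itself when the timeline finishes; Haunt_1 is an empty stub.
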(event Custom|Haunt_1)

(event Collision|EventActorBeginOverlap
  (params (OtherActor :type Actor%20Object%20Reference)))

(event EventTick
  (params (DeltaSeconds :type Float%20%28single-precision%29)))

(event EventGhostWalkDownStairs
  (bind _movepath (Variables|Default|GetMovePath))
  (bind _spline (Variables|Default|GetSpline))
  (bind _pathway (Variables|/Game/Ghost/BP_GhostTracking.BP_GhostTracking_C|GetPathway _spline))
  (Development|SetHiddeninGame (Variables|Default|GetSkeletalMesh) false false)
  (Components|Timeline|SetPlayRate _movepath (/ 1.0 (Variables|Default|GetDuration)))
  (Components|Timeline|SetNewTime _movepath (Variables|Default|GetMovement%20Offset))
  (bind _movement (Timeline|MovePath Play)
    (:Update
      (Variables|Default|SetMovement _movement)
      (Transformation|SetActorLocationAndRotation (Spline|GetLocationatDistanceAlongSpline _pathway (Math|Float|Lerp 0.0 (Spline|GetSplineLength _pathway) (Variables|Default|GetMovement)) "World") (Spline|GetRotationatDistanceAlongSpline _pathway (Math|Float|Lerp 0.0 (Spline|GetSplineLength _pathway) (Variables|Default|GetMovement)) "Local")))
    (:Finished
      (Actor|DestroyActor))))

(event EventBeginPlay
  (Development|SetHiddeninGame (Variables|Default|GetSkeletalMesh) true false))

(fn ConstructionScript)