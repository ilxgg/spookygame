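; Player character Blueprint that drives a stress screen effect, the pause menu and key rebinding.
; BeginPlay installs a dynamic vignette material in the camera's post-process settings and applies initial timed stress, while Tick feeds StressComponent's level into that material.
; The Menu action toggles pause, the MenuRef widget, cursor and input mode.
; While RebindKeyActive is set, an any-key listener forwards the pressed key to the menu as a new binding.
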(event EventBeginPlay
  (bind _returnvalue (Rendering|Material|CreateDynamicMaterialInstance "/Game/Level/Materials/PostProcess/StressVignette.StressVignette" "StressEffect" "None" :!class /Script/Engine.KismetMaterialLibrary))
  (bind _output_get (Variables|Default|SetStressMatPP _returnvalue))
  (Variables|/Script/Engine.CameraComponent|SetPostProcessSettings (Variables|Default|GetCamera) (Utilities|Struct|MakePostProcessSettings 0.1 0.1 (Utilities|Struct|MakeWeightedBlendables (Utilities|Array|MakeArray (Utilities|Struct|MakeWeightedBlendable 1.0 _output_get)))))
  (Class|PlayerCharacter|ApplyStress 8e+01 3.0))

(event Collision|EventActorBeginOverlap
  (params (OtherActor :type Actor%20Object%20Reference)))

(event EventTick
  (params (DeltaSeconds :type Float%20%28single-precision%29))
  (bind _returnvalue (Class|StressComponent|GetCurrentStress (Variables|Default|GetStressComponent)))
  (Rendering|Material|SetScalarParameterValue (Variables|Default|GetStressMatPP) "StressLevel" _returnvalue :!class /Script/Engine.MaterialInstanceDynamic))

(event Input|ActionEvents|InputActionMenu
  (params (Key :type Key%20Structure :default "None"))
  (bind _returnvalue (Game|GetPlayerController 0))
  (bind _returnvalue_2 (Game|GetPlayerController 0))
  (:Pressed
    (Utilities|IsValid (Variables|Default|GetMenuRef)
      (:Is%20Valid
        (if (Variables|Default|GetMenuOpen)
          (Variables|Default|SetMenuOpen false)
          (Viewport|RemoveAllWidgets)
          (Input|SetInputModeGameOnly _returnvalue)
          (Variables|/Script/Engine.PlayerController|SetbShowMouseCursor _returnvalue false)
          (Game|SetGamePaused false)
          (else
            (Variables|Default|SetMenuOpen true)
            (Input|SetInputModeGameandUI _returnvalue_2 0 "LockAlways" true)
            (UserInterface|Viewport|AddtoViewport (Variables|Default|GetMenuRef) 0)
            (Variables|/Script/Engine.PlayerController|SetbShowMouseCursor _returnvalue_2 true)
            (Game|SetGamePaused true)))))))

(event Input|KeyboardEvents|AnyKey
  (params (Key :type Key%20Structure :default "None"))
  (:Pressed
    (if (Variables|Default|GetRebindKeyActive)
      (Default|CallOnKeyRebind (Variables|Default|GetMenuRef) Key (Variables|Default|GetNewKeybindAction))
      (Variables|Default|SetRebindKeyActive false)
      (Variables|Default|SetNewKeybindAction "NewEnumerator5"))))

(fn ConstructionScript)